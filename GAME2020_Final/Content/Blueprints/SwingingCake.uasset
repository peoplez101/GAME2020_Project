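; SwingingCake is an actor that swings back and forth by rotating around its yaw axis.
; Each Tick adds SwingAmount to SwingDegree and applies a scaled SwingDegree as a local rotation increment, so the counter acts as angular velocity.
; SwingAmount flips sign at the counter's positive and negative limits, easing each reversal.
; Motion is stepped per frame without delta time, so it depends on frame rate.
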(event `self.ReceiveTick`
  (params (DeltaSeconds :type "Float (single-precision)"))
  (bind _output_get (set `self.SwingDegree` (+ (`self.SwingDegree`) (`self.SwingAmount`))))
  (`self.K2_AddActorLocalRotation` (`KismetMathLibrary.MakeRotator` 0.0 0.0 (* _output_get 0.01)))
  (if (>= (`self.SwingDegree`) 90.0)
    (set `self.SwingAmount` -0.5)
    (elif (<= (`self.SwingDegree`) -90.0)
      (set `self.SwingAmount` 0.5))))

(fn `UserConstructionScript`)